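; Player character Blueprint that handles axis-based movement and a ground-checked jump.
; Jump input fires a debug-drawn Visibility line trace down from the Cube component by Distance, jumping only if the hit actor is tagged Ground and printing either result.
; MoveForward and MoveRight add movement input along control rotation vectors.
; Tick copies PlayerSpeed into the movement component's MaxWalkSpeed every frame.
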(event EventTick
  (params (DeltaSeconds :type Float%20%28single-precision%29))
  ;[1 1 1] MovementSpeed
  (Variables|/Script/Engine.CharacterMovementComponent|SetMaxWalkSpeed (Variables|Character|GetCharacterMovement) (Variables|Default|GetPlayer%20Speed)))

(event Input|ActionEvents|InputActionJump
  (params (Key :type Key%20Structure :default "None"))
  (bind _cube (Variables|Default|GetCube))
  (bind _returnvalue (Transformation|GetWorldLocation _cube))
  ;[1 1 1] Jump/LineTrace
  (:Pressed
    (bind _outhit (Collision|LineTraceByChannel _returnvalue (+ _returnvalue (* "0, 0,-1.000000" (Variables|Default|GetDistance))) "TraceTypeQuery1" false 0 "ForDuration"))
    (if (Actor|ActorHasTag (.HitActor (Collision|BreakHitResult _outhit)) "Ground")
      (Development|PrintString "Jumping on Ground")
      (Character|Jump)
      (else
        (Development|PrintString "Not on Ground")))))

(event Input|AxisEvents|InputAxisMoveForward
  (params (AxisValue :type Float%20%28single-precision%29))
  ;[1 1 1] MoveForward/Backward
  (Pawn|Input|AddMovementInput (Math|Vector|GetForwardVector (Pawn|GetControlRotation :!class /Script/Engine.Pawn)) AxisValue false))

(event Input|AxisEvents|InputAxisMoveRight
  (params (AxisValue :type Float%20%28single-precision%29))
  ;[1 1 1] MoveRight/Left
  (Pawn|Input|AddMovementInput (Math|Vector|GetRightVector (Pawn|GetControlRotation :!class /Script/Engine.Pawn)) AxisValue false))

(fn ConstructionScript)